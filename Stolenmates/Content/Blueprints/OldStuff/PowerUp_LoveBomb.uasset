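; Love Bomb power-up that stuns players in two stages, extending a parent power-up's overlap behavior.
; When a non-owner player holding the heart begins overlapping the main collision, it stuns that player and arms itself through IsEnemy.
; Once armed, any non-owner player who begins overlapping the range-stun collision gets a shorter stun, and IsDone is set.
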(event `self.ReceiveTick`
  (params (DeltaSeconds :type "Float (single-precision)")))

(event `self.Collision.OnComponentBeginOverlap`
  (params (OverlappedComponent :type "PrimitiveComponent Object Reference") (OtherActor :type "Actor Object Reference") (OtherComp :type "PrimitiveComponent Object Reference") (OtherBodyIndex :type Integer) (bFromSweep :type Boolean) (SweepResult :type "HitResult Structure (by ref)"))
  (`parent.ReceiveActorBeginOverlap` OtherActor)
  (if (not (== (`self.GetOwner`) OtherActor))
    (bind _asstolenmates_player (cast `StolenmatesPlayer` OtherActor))
    (if (`StolenmatesPlayer.hasHeart` _asstolenmates_player)
      (set `self.is enemy` true)
      (`StolenmatesPlayer.StunPlayer` _asstolenmates_player 3.0))))

(event `self.rangestun_collision.OnComponentBeginOverlap`
  (params (OverlappedComponent :type "PrimitiveComponent Object Reference") (OtherActor :type "Actor Object Reference") (OtherComp :type "PrimitiveComponent Object Reference") (OtherBodyIndex :type Integer) (bFromSweep :type Boolean) (SweepResult :type "HitResult Structure (by ref)"))
  (if (`self.is enemy`)
    (if (not (== OtherActor (`self.GetOwner`)))
      (bind _asstolenmates_player (cast `StolenmatesPlayer` OtherActor))
      (`StolenmatesPlayer.StunPlayer` _asstolenmates_player 1.5)
      (set `self.is done` true))))

(fn `UserConstructionScript`
  (`parent.UserConstructionScript`))