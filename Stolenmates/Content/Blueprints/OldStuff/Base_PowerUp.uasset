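; Base power-up actor with empty CallPowerUp and Callbaseclass functions, the former taking a player and a power-up.
; Tick acts only when IsEnemy is set, first destroying the collision and mesh components once and flagging that as done.
; On later ticks it destroys the whole actor once IsDone is true, a flag this Blueprint never sets itself.
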(event `self.ReceiveTick`
  (params (DeltaSeconds :type "Float (single-precision)"))
  (if (`self.is enemy`)
    (if (`self.is collision destroyed`)
      (if (`self.is done`)
        (`self.K2_DestroyActor`))
      (else
        (`ActorComponent.K2_DestroyComponent` (`self.Collision`))
        (`ActorComponent.K2_DestroyComponent` (`self.mesh`))
        (set `self.is collision destroyed` true)))))

(fn `Call_Power_Up`
  (params (Player :type "Actor Object Reference") (Power_Up :type Integer)))

(fn `callbaseclass`)

(fn `UserConstructionScript`)