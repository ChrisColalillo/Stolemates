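; Catfish power-up actor that stuns any overlapping Stolenmates player other than its owner.
; On overlap it runs the parent handler, then compares the other actor with its owner to set an enemy flag.
; For non-owners it casts to StolenmatesPlayer and calls StunPlayer with the stun time, toggling a done flag around the call.
; The construction script only calls the parent.
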(event `self.ReceiveActorBeginOverlap`
  (params (OtherActor :type "Actor Object Reference"))
  (`parent.ReceiveActorBeginOverlap` OtherActor)
  (if (== OtherActor (`self.GetOwner`))
    (set `self.is enemy` false)
    (else
      (bind _output_get (set `self.is enemy` true))
      (if _output_get
        (set `self.is done` false)
        (bind _asstolenmates_player (cast `StolenmatesPlayer` OtherActor))
        (`StolenmatesPlayer.StunPlayer` _asstolenmates_player (`self.stun_time`))
        (set `self.is done` true)))))

(fn `UserConstructionScript`
  (`parent.UserConstructionScript`))