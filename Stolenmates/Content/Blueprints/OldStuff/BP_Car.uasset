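; BP_Car is an actor that travels along the spline of a referenced track.
; On BeginPlay, if ActiveCart is set, it plays a timeline with a rate derived from Duration, starting at CarStartOffset.
; Each update maps the timeline alpha to a distance along UsefulSpline and moves the actor to that world location.
; Only location is sampled from the spline, so the car does not orient to the track.
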(event `self.ReceiveBeginPlay`
  (if (`self.ActiveCart`)
    (`self.MoveCar`)))

(event `MoveCar`
  (`TimelineComponent.SetPlayRate` (`self.CarMovement`) (/ 1.0 (`self.Duration`)))
  (`TimelineComponent.SetNewTime` (`self.CarMovement`) (`self.CarStartOffset`))
  (bind (_direction _newtrack_1) (`Timeline|CarMovement`)
    (:`Update`
      (set `self.Alpha` _newtrack_1)
      (`self.K2_SetActorLocationAndRotation` (`SplineComponent.GetLocationAtDistanceAlongSpline` (`/Game/Blueprints/OldStuff/BP_Track.UsefulSpline` (`self.TrackRef`)) (`KismetMathLibrary.Lerp` 0.0 (`SplineComponent.GetSplineLength` (`/Game/Blueprints/OldStuff/BP_Track.UsefulSpline` (`self.TrackRef`))) (`self.Alpha`)) "World")))))

(fn `UserConstructionScript`)