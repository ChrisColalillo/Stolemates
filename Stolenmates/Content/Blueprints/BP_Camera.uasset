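; Shared multiplayer camera for up to four BP_Player actors, set as the view target of all player controllers.
; A looping timer runs position and zoom logic matched to the player count.
; The actor eases toward the midpoint of the two farthest-apart players within clamped bounds, tightening the X limit as they spread.
; Spring arm length eases toward the largest screen-aspect-weighted player offset, clamped, with a fixed length below LockDistance.
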(event `self.ReceiveBeginPlay`
  (`|ExecutionSequence`
    (:`then_0`
      (`KismetSystemLibrary.Delay` 0.1)
      (bind _outactors (`GameplayStatics.GetAllActorsOfClass` "/Game/Blueprints/BP_Player.BP_Player_C"))
      (for _array_element _outactors
        (`KismetArrayLibrary.Array_AddUnique` (`self.PlayersReference`) _array_element)))
    (:`then_1`
      (`KismetSystemLibrary.Delay` 0.1)
      (`self.Class Setup`)
      (`KismetSystemLibrary.K2_SetTimer` null "UpdateCamera" 0.001 true))))

(event `UpdateCamera`
  (switch `int` (`KismetArrayLibrary.Array_Length` (`self.PlayersReference`))
    (:`1`
      (`self.SetCameraPos1`))
    (:`2`
      (`self.SetPlayerDistance02`)
      (`self.SetCameraPos2`))
    (:`3`
      (`self.SetPlayerDistance03`)
      (`self.SetCameraPos3`))
    (:`4`
      (`self.SetPlayerDistance04`)
      (`self.SetCameraPos4`))))

(fn `CameraOffsetx`
  (params (`X of MiddleDistanceOfFarPlayers` :type "Float (double-precision)") (LargestDistanceBetweenPlayers :type "Float (double-precision)"))
  (returns (`Camera Offset (x)` :type "Float (double-precision)"))
  (return 0.0))

(fn `CameraOffsety`
  (params (`Middle Point (y)` :type "Float (double-precision)"))
  (returns (`Camera Offset (y)` :type "Float (double-precision)"))
  (return (* (+ (`KismetMathLibrary.MultiplyMultiply_FloatFloat` (/ (`KismetMathLibrary.Abs` `Middle Point (y)`) 1e-05) (/ 1.0 3.0)) 45.0) -1.0)))

(fn `Class Setup`
  (bind _outactors (`GameplayStatics.GetAllActorsOfClass` "/Script/Engine.PlayerController"))
  (`PlayerController.SetViewTargetWithBlend` _outactors self 0.0 "VTBlend_Linear" 0.0 false)
  (for (_array_element _array_index) (`self.PlayersReference`)
    (switch `int` _array_index
      (:`0`
        (set `self.P1` _array_element))
      (:`1`
        (set `self.P2` _array_element))
      (:`2`
        (set `self.P3` _array_element))
      (:`3`
        (set `self.P4` _array_element)))))

(fn `FarthestX&Y`
  (returns (`Zoom Factor` :type "Float (double-precision)"))
  (bind (_currentposition_x _currentposition_y) (`KismetMathLibrary.BreakVector` (`self.CurrentPosition`)))
  (bind (_returnvalue_x _returnvalue_y) (`KismetMathLibrary.BreakVector` (`self.K2_GetActorLocation` (`self.P4`))))
  (bind (_returnvalue_x_2 _returnvalue_y_2) (`KismetMathLibrary.BreakVector` (`self.K2_GetActorLocation` (`self.P1`))))
  (bind (_returnvalue_x_3 _returnvalue_y_3) (`KismetMathLibrary.BreakVector` (`self.K2_GetActorLocation` (`self.P2`))))
  (bind (_returnvalue_x_4 _returnvalue_y_4) (`KismetMathLibrary.BreakVector` (`self.K2_GetActorLocation` (`self.P3`))))
  (bind _output_get (set `self.Largest X Value` (`.MaxValue` (`KismetMathLibrary.MaxOfFloatArray` (`|MakeArray` (`KismetMathLibrary.Abs` (- _returnvalue_x_2 _currentposition_x)) (`KismetMathLibrary.Abs` (- _returnvalue_x_3 _currentposition_x)) (`KismetMathLibrary.Abs` (- _returnvalue_x_4 _currentposition_x)) (`KismetMathLibrary.Abs` (- _returnvalue_x _currentposition_x)))))))
  (bind _output_get_2 (set `self.Largest Y Value` (`.MaxValue` (`KismetMathLibrary.MaxOfFloatArray` (`|MakeArray` (`KismetMathLibrary.Abs` (- _returnvalue_y_2 _currentposition_y)) (`KismetMathLibrary.Abs` (- _returnvalue_y_3 _currentposition_y)) (`KismetMathLibrary.Abs` (- _returnvalue_y_4 _currentposition_y)) (`KismetMathLibrary.Abs` (- _returnvalue_y _currentposition_y)))))))
  (return (`.MaxValue` (`KismetMathLibrary.MaxOfFloatArray` (`|MakeArray` (/ _output_get_2 540.0) (/ _output_get 960.0))))))

(fn `FindFarthestPlayers`
  (returns (X :type "Float (double-precision)") (Y :type "Float (double-precision)") (Z :type "Float (double-precision)") (MiddlePointOfFarPlayers :type "Vector Structure") (MaxValue :type "Float (double-precision)"))
  (bind _p1 (`self.P1`))
  (bind _p2 (`self.P2`))
  (bind _p3 (`self.P3`))
  (bind _p4 (`self.P4`))
  (bind _p3_2 (`self.P3`))
  (bind _p4_2 (`self.P4`))
  (bind _p1_2 (`self.P1`))
  (bind _p2_2 (`self.P2`))
  (bind (_returnvalue_x _returnvalue_y _returnvalue_z) (`KismetMathLibrary.BreakVector` (/ (+ (`self.K2_GetActorLocation` (`self.Target1`)) (`self.K2_GetActorLocation` (`self.Target 2`))) 2.0)))
  (bind _output_get (set `self.PlayerDistances` (`|MakeArray` (`self.GetDistanceTo` _p1_2 _p2_2) (`self.GetDistanceTo` _p1_2 _p3) (`self.GetDistanceTo` _p1_2 _p4) (`self.GetDistanceTo` _p2_2 _p3) (`self.GetDistanceTo` _p2_2 _p4) (`self.GetDistanceTo` _p3 _p4))))
  (bind (_indexofmaxvalue _maxvalue) (`KismetMathLibrary.MaxOfFloatArray` _output_get))
  (switch `int` _indexofmaxvalue
    (:`0`
      (set `self.Target1` _p1)
      (set `self.Target 2` _p2))
    (:`1`
      (set `self.Target1` _p1)
      (set `self.Target 2` _p3_2))
    (:`2`
      (set `self.Target1` _p1)
      (set `self.Target 2` _p4_2))
    (:`3`
      (set `self.Target1` _p2)
      (set `self.Target 2` _p3_2))
    (:`4`
      (set `self.Target1` _p2)
      (set `self.Target 2` _p4_2))
    (:`5`
      (set `self.Target1` _p3_2)
      (set `self.Target 2` _p4_2)))
  (return _returnvalue_x _returnvalue_y _returnvalue_z (`KismetMathLibrary.MakeVector` _returnvalue_x _returnvalue_y _returnvalue_z) _maxvalue))

(fn `SetCameraPos1`
  (set `SpringArmComponent.TargetArmLength` (`self.MinArmLength`) (`self.SpringArm`))
  (set `self.CurrentPosition` (`self.K2_GetActorLocation` (`self.P1`)))
  (`self.K2_SetActorLocation` (`KismetMathLibrary.VInterpTo` (`self.PreviousPosition`) (`self.CurrentPosition`) (`GameplayStatics.GetWorldDeltaSeconds`) (`self.InterpSpeed`)))
  (set `self.PreviousPosition` (`self.K2_GetActorLocation`)))

(fn `SetCameraPos2`
  (bind (_returnvalue_x _returnvalue_y _returnvalue_z) (`KismetMathLibrary.BreakVector` (/ (+ (`self.K2_GetActorLocation` (`self.P1`)) (`self.K2_GetActorLocation` (`self.P2`))) 2.0)))
  (bind _output_get (set `self.PlayerDistances` (`|MakeArray` (`self.GetDistanceTo` (`self.P1`) (`self.P2`)))))
  (set `self.CurrentPosition` (`KismetMathLibrary.MakeVector` (`KismetMathLibrary.FClamp` _returnvalue_x -1000.0 (`KismetMathLibrary.FClamp` (- 2000.0 (* (/ (`.MaxValue` (`KismetMathLibrary.MaxOfFloatArray` _output_get)) 8000.0) 6000.0)) -1000.0 2000.0)) (`KismetMathLibrary.FClamp` _returnvalue_y -2000.0 2000.0) _returnvalue_z))
  (`self.K2_SetActorLocation` (`KismetMathLibrary.VInterpTo` (`self.PreviousPosition`) (`self.CurrentPosition`) (`GameplayStatics.GetWorldDeltaSeconds`) (`self.InterpSpeed`)))
  (set `self.PreviousPosition` (`self.K2_GetActorLocation`)))

(fn `SetCameraPos3`
  (bind _p1 (`self.P1`))
  (bind _p2 (`self.P2`))
  (bind _p3 (`self.P3`))
  (bind _p3_2 (`self.P3`))
  (bind _p1_2 (`self.P1`))
  (bind _p2_2 (`self.P2`))
  (bind (_returnvalue_x _returnvalue_y _returnvalue_z) (`KismetMathLibrary.BreakVector` (/ (+ (`self.K2_GetActorLocation` (`self.Target1`)) (`self.K2_GetActorLocation` (`self.Target 2`))) 2.0)))
  (bind _output_get (set `self.PlayerDistances` (`|MakeArray` (`self.GetDistanceTo` _p1_2 _p2_2) (`self.GetDistanceTo` _p1_2 _p3) (`self.GetDistanceTo` _p2_2 _p3))))
  (bind (_indexofmaxvalue _maxvalue) (`KismetMathLibrary.MaxOfFloatArray` _output_get))
  (switch `int` _indexofmaxvalue
    (:`0`
      (set `self.Target1` _p1)
      (set `self.Target 2` _p2))
    (:`1`
      (set `self.Target1` _p1)
      (set `self.Target 2` _p3_2))
    (:`2`
      (set `self.Target1` _p2)
      (set `self.Target 2` _p3_2)))
  (set `self.CurrentPosition` (`KismetMathLibrary.MakeVector` (`KismetMathLibrary.FClamp` _returnvalue_x -1000.0 (`KismetMathLibrary.FClamp` (- 2000.0 (* (/ _maxvalue 8000.0) 6000.0)) -1000.0 2000.0)) (`KismetMathLibrary.FClamp` _returnvalue_y -2000.0 2000.0) _returnvalue_z))
  (`self.K2_SetActorLocation` (`KismetMathLibrary.VInterpTo` (`self.PreviousPosition`) (`self.CurrentPosition`) (`GameplayStatics.GetWorldDeltaSeconds`) (`self.InterpSpeed`)))
  (set `self.PreviousPosition` (`self.K2_GetActorLocation`)))

(fn `SetCameraPos4`
  (bind (_x _y _z _middlepointoffarplayers _maxvalue) (`self.FindFarthestPlayers`))
  (set `self.CurrentPosition` (`KismetMathLibrary.MakeVector` (`KismetMathLibrary.FClamp` _x -1000.0 (`KismetMathLibrary.FClamp` (- 2000.0 (* (/ _maxvalue 8000.0) 6000.0)) -1000.0 2000.0)) (`KismetMathLibrary.FClamp` _y -2000.0 2000.0) _z))
  (`self.K2_SetActorLocation` (`KismetMathLibrary.VInterpTo` (`self.PreviousPosition`) (`self.CurrentPosition`) (`GameplayStatics.GetWorldDeltaSeconds`) (`self.InterpSpeed`)))
  (set `self.PreviousPosition` (`self.K2_GetActorLocation`)))

(fn `SetPlayerDistance02`
  (bind _returnvalue (`GameplayStatics.GetWorldDeltaSeconds`))
  (bind (_currentposition_x _currentposition_y) (`KismetMathLibrary.BreakVector` (`self.CurrentPosition`)))
  (bind _springarm (`self.SpringArm`))
  (bind (_returnvalue_x _returnvalue_y) (`KismetMathLibrary.BreakVector` (`self.K2_GetActorLocation` (`self.P1`))))
  (bind (_returnvalue_x_2 _returnvalue_y_2) (`KismetMathLibrary.BreakVector` (`self.K2_GetActorLocation` (`self.P2`))))
  (bind _targetarmlength (`SpringArmComponent.TargetArmLength` _springarm))
  (bind _output_get (set `self.Largest X Value` (`.MaxValue` (`KismetMathLibrary.MaxOfFloatArray` (`|MakeArray` (`KismetMathLibrary.Abs` (- _returnvalue_x _currentposition_x)) (`KismetMathLibrary.Abs` (- _returnvalue_x_2 _currentposition_x)))))))
  (bind _output_get_2 (set `self.Largest Y Value` (`.MaxValue` (`KismetMathLibrary.MaxOfFloatArray` (`|MakeArray` (`KismetMathLibrary.Abs` (- _returnvalue_y _currentposition_y)) (`KismetMathLibrary.Abs` (- _returnvalue_y_2 _currentposition_y)))))))
  (bind _returnvalue_2 (* (`.MaxValue` (`KismetMathLibrary.MaxOfFloatArray` (`|MakeArray` (/ _output_get_2 540.0) (/ _output_get 960.0)))) 800.0))
  (if (<= _returnvalue_2 (`self.LockDistance`))
    (set `SpringArmComponent.TargetArmLength` (`KismetMathLibrary.FInterpTo` _targetarmlength 700.0 _returnvalue 0.33) _springarm)
    (else
      (set `SpringArmComponent.TargetArmLength` (`KismetMathLibrary.FInterpTo` _targetarmlength (`KismetMathLibrary.FClamp` _returnvalue_2 (`self.MinArmLength`) (`self.MaxArmLength`)) _returnvalue 0.33) _springarm))))

(fn `SetPlayerDistance03`
  (bind _returnvalue (`GameplayStatics.GetWorldDeltaSeconds`))
  (bind (_currentposition_x _currentposition_y) (`KismetMathLibrary.BreakVector` (`self.CurrentPosition`)))
  (bind _springarm (`self.SpringArm`))
  (bind (_returnvalue_x _returnvalue_y) (`KismetMathLibrary.BreakVector` (`self.K2_GetActorLocation` (`self.P1`))))
  (bind (_returnvalue_x_2 _returnvalue_y_2) (`KismetMathLibrary.BreakVector` (`self.K2_GetActorLocation` (`self.P2`))))
  (bind (_returnvalue_x_3 _returnvalue_y_3) (`KismetMathLibrary.BreakVector` (`self.K2_GetActorLocation` (`self.P3`))))
  (bind _targetarmlength (`SpringArmComponent.TargetArmLength` _springarm))
  (bind _output_get (set `self.Largest X Value` (`.MaxValue` (`KismetMathLibrary.MaxOfFloatArray` (`|MakeArray` (`KismetMathLibrary.Abs` (- _returnvalue_x _currentposition_x)) (`KismetMathLibrary.Abs` (- _returnvalue_x_2 _currentposition_x)) (`KismetMathLibrary.Abs` (- _returnvalue_x_3 _currentposition_x)))))))
  (bind _output_get_2 (set `self.Largest Y Value` (`.MaxValue` (`KismetMathLibrary.MaxOfFloatArray` (`|MakeArray` (`KismetMathLibrary.Abs` (- _returnvalue_y _currentposition_y)) (`KismetMathLibrary.Abs` (- _returnvalue_y_2 _currentposition_y)) (`KismetMathLibrary.Abs` (- _returnvalue_y_3 _currentposition_y)))))))
  (bind _returnvalue_2 (* (`.MaxValue` (`KismetMathLibrary.MaxOfFloatArray` (`|MakeArray` (/ _output_get_2 540.0) (/ _output_get 960.0)))) 800.0))
  (if (<= _returnvalue_2 (`self.LockDistance`))
    (set `SpringArmComponent.TargetArmLength` (`KismetMathLibrary.FInterpTo` _targetarmlength 700.0 _returnvalue 0.33) _springarm)
    (else
      (set `SpringArmComponent.TargetArmLength` (`KismetMathLibrary.FInterpTo` _targetarmlength (`KismetMathLibrary.FClamp` _returnvalue_2 (`self.MinArmLength`) (`self.MaxArmLength`)) _returnvalue 0.33) _springarm))))

(fn `SetPlayerDistance04`
  (bind _returnvalue (`GameplayStatics.GetWorldDeltaSeconds`))
  (bind _springarm (`self.SpringArm`))
  (bind _targetarmlength (`SpringArmComponent.TargetArmLength` _springarm))
  (bind _zoom_factor (`self.FarthestX&Y`))
  (bind _returnvalue_2 (* _zoom_factor 800.0))
  (if (<= _returnvalue_2 (`self.LockDistance`))
    (set `SpringArmComponent.TargetArmLength` (`KismetMathLibrary.FInterpTo` _targetarmlength 700.0 _returnvalue 0.33) _springarm)
    (else
      (set `SpringArmComponent.TargetArmLength` (`KismetMathLibrary.FInterpTo` _targetarmlength (`KismetMathLibrary.FClamp` _returnvalue_2 (`self.MinArmLength`) (`self.MaxArmLength`)) _returnvalue 0.33) _springarm))))

(fn `UserConstructionScript`)