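; BP_Tracking is an AI-moved projectile-like pawn that stuns players it touches, other than its Creator.
; On BeginPlay it uses SimpleMoveToLocation toward the Target's position at that moment, without updating it afterward, then destroys itself after five seconds.
; Its Box overlap casts to BP_Player, skips the Creator, calls StunPlayer on anyone else and destroys itself.
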(event `self.ReceiveBeginPlay`
  (`AIBlueprintHelperLibrary.SimpleMoveToLocation` (`self.GetController`) (`self.K2_GetActorLocation` (`self.Target`)))
  (`KismetSystemLibrary.Delay` 5.0)
  (`self.K2_DestroyActor`))

(event `self.Box.OnComponentBeginOverlap`
  (params (OverlappedComponent :type "PrimitiveComponent Object Reference") (OtherActor :type "Actor Object Reference") (OtherComp :type "PrimitiveComponent Object Reference") (OtherBodyIndex :type Integer) (bFromSweep :type Boolean) (SweepResult :type "HitResult Structure (by ref)"))
  (bind _asbp_player (cast `/Game/Blueprints/BP_Player` OtherActor))
  (if (!= _asbp_player (`self.Creator`))
    (`StolenmatesPlayer.StunPlayer` _asbp_player 3.0)
    (`self.K2_DestroyActor`)))

(fn `UserConstructionScript`)