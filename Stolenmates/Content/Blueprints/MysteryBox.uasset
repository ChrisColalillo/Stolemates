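; Mystery box pickup that removes its cube when a BP_Player overlaps it, then picks a random effect.
; Sliding lowers other players' ground friction temporarily, while SpeedBoost briefly raises the collector's walk speed; both then destroy the box.
; Love Bomb only prints that it is not working.
; Each branch check re-rolls the random number, so odds are uneven and a pickup can give no effect.
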(event `self.collision.OnComponentBeginOverlap`
  (params (OverlappedComponent :type "PrimitiveComponent Object Reference") (OtherActor :type "Actor Object Reference") (OtherComp :type "PrimitiveComponent Object Reference") (OtherBodyIndex :type Integer) (bFromSweep :type Boolean) (SweepResult :type "HitResult Structure (by ref)"))
  (bind _returnvalue (`KismetMathLibrary.RandomIntegerInRange` 0 2))
  (bind _speedboostvalue (`self.SpeedBoostValue`))
  (bind _asbp_player (cast `/Game/Blueprints/BP_Player` OtherActor))
  (`ActorComponent.K2_DestroyComponent` (`self.Cube`))
  (if (== _returnvalue 0)
    (`KismetSystemLibrary.PrintString` "Sliding into the DMs")
    ;[1 1 1] Sliding
    (bind _outactors (`GameplayStatics.GetAllActorsOfClass` "/Game/Blueprints/BP_Player.BP_Player_C"))
    (for _array_element _outactors
      (if (!= _array_element OtherActor)
        (set `CharacterMovementComponent.GroundFriction` 0.5 (`Character.CharacterMovement` _array_element))
        (`KismetSystemLibrary.Delay` 10.0)
        (for _array_element_2 _outactors
          (set `CharacterMovementComponent.GroundFriction` 8.0 (`Character.CharacterMovement` _array_element_2))
          (`KismetSystemLibrary.Delay` 0.1)
          (`self.K2_DestroyActor` :!label _label))))
    (elif (== _returnvalue 1)
      (`KismetSystemLibrary.PrintString` "Love Bomb(Not Currently Working)")
      (elif (== _returnvalue 2)
        ;[1 1 1] SpeedBoost
        (`KismetSystemLibrary.PrintString` "SpeedBoost")
        (bind _charactermovement (`Character.CharacterMovement` _asbp_player))
        (bind _maxwalkspeed (`CharacterMovementComponent.MaxWalkSpeed` _charactermovement))
        (set `CharacterMovementComponent.MaxWalkSpeed` (+ _maxwalkspeed _speedboostvalue) _charactermovement)
        (`KismetSystemLibrary.Delay` 5.0)
        (set `CharacterMovementComponent.MaxWalkSpeed` (- _maxwalkspeed _speedboostvalue) _charactermovement)
        (goto _label)))))

(fn `Random Int`
  (returns (RandomInt :type Integer))
  (return (`KismetMathLibrary.RandomIntegerInRange` 0 2)))

(fn `UserConstructionScript`)