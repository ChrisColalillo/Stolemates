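; Game mode Blueprint that shows the Win widget at game over, switching the player to UI-only input with a visible cursor.
; SpawnPowerUp, GeneratePowerup and LoadHud are empty events, with related logic left in disconnected, never-run chains.
; Those chains would create a player-count HUD and run an EQS query that spawns a MysteryBox at every returned location, marked as temporary debug.
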(event `self.SpawnPowerUp`)

(event `GeneratePowerup`
  (params (QueryInstance :type "EnvQueryInstanceBlueprintWrapper Object Reference") (QueryStatus :type "EEnvQueryStatus Enum" :default "Processing")))

(event `self.LoadHud`
  (params (PlayerController :type "PlayerController Object Reference")))

(event `self.GameOverHud`
  (params (PlayerController :type "PlayerController Object Reference"))
  (bind _returnvalue (`|CreateWidget` "/Game/Blueprints/Win.Win_C"))
  (`UserWidget.AddToViewport` _returnvalue 0)
  (`WidgetBlueprintLibrary.SetInputMode_UIOnlyEx` PlayerController _returnvalue)
  (set `PlayerController.bShowMouseCursor` true PlayerController))

(fn `UserConstructionScript`)