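; BoxSpawn_Loc is a spawn point that keeps respawning a mystery box at the location of its ChildActor component.
; From BeginPlay it loops, waiting a random time between configurable bounds, then spawning a box and attaching it to that component.
; While occupied, it polls the component's first child every tenth of a second and clears HasBox when none remains, triggering the next timed spawn.
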(event `self.ReceiveBeginPlay`
  (bind _childactor (`self.ChildActor`))
  (if (`self.HasBox`) :!label _label
    (if (== (`SceneComponent.GetChildComponent` (`self.ChildActor`) 0) null)
      (set `self.HasBox` false)
      (`KismetSystemLibrary.Delay` 0.1)
      (goto _label)
      (else
        (`KismetSystemLibrary.Delay` 0.1)
        (goto _label)))
    (else
      (`KismetSystemLibrary.Delay` (`KismetMathLibrary.RandomFloatInRange` (`self.SpawnTimeMin`) (`self.SpawnTimeMax`)))
      (bind _returnvalue (`|SpawnActorFromClass` "/Game/Blueprints/MysteryBox.MysteryBox_C" (`SceneComponent.K2_GetComponentToWorld` _childactor) "AdjustIfPossibleButAlwaysSpawn" "OverrideRootScale" null null))
      (set `self.HasBox` true)
      (`self.K2_AttachToComponent` _returnvalue _childactor "None" "KeepWorld" "KeepWorld" "KeepWorld" false)
      (goto _label))))

(fn `UserConstructionScript`)