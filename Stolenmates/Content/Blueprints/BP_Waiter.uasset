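; BP_Waiter is a pawn that walks an endless patrol through the actors in its Waypoint01 array.
; BeginPlay starts the custom Patrol event, which uses AIMoveTo toward the waypoint at CurrentTarget.
; On success it advances the index, wrapping to the first at the end, pauses briefly and calls Patrol again.
; A failed move has no handler, so the loop stops there.
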(event `self.ReceiveBeginPlay`
  (`self.Patrol`))

(event `Patrol`
  (bind _waypoint01 (`self.Waypoint01`))
  (bind _currenttarget (`self.CurrentTarget`))
  (bind _returnvalue (+ _currenttarget 1))
  (`|AIMoveTo` self (0.0 0.0 0.0) (`|GetArrayItem` _waypoint01 _currenttarget)
    (:`OnSuccess`
      (if (>= _returnvalue (`KismetArrayLibrary.Array_Length` _waypoint01))
        (set `self.CurrentTarget` 0)
        (else
          (set `self.CurrentTarget` _returnvalue)))
      (`KismetSystemLibrary.Delay` 1.5)
      (`self.Patrol`))))

(fn `UserConstructionScript`)