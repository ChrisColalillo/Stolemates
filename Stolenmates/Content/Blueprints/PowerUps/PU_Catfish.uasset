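; PU_Catfish is a catfish trap power-up that stuns players who run into it.
; On activation, the server traces down from the activating player and picks a random yaw.
; A multicast then places the enlarged catfish at that point, arms it and unpauses its animation.
; Server-side box overlap ignores the activating player, marks other non-immune players as catfished, stuns them, and destroys the trap even if they are immune.
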(event `MulticastActivateCatfishVisuals`
  (params (CatfishLocation :type "Vector Structure") (CatfishRotation :type "Rotator Structure") (CatfishScale :type "Vector Structure") (`Target Catfish` :type "Actor Object Reference"))
  (`self.K2_SetActorTransform` `Target Catfish` (`KismetMathLibrary.MakeTransform` CatfishLocation (`KismetMathLibrary.MakeRotator` 0.0 0.0 CatfishRotation_Yaw) (2.0 2.0 2.0)) false false)
  (set `self.Active` true)
  (set `SkeletalMeshComponent.bPauseAnims` false (`self.SkeletalMesh`)))

(event `Activate`
  (params (TargetPlayer :type "/Game/Blueprints/BP_Player Object Reference") (StunDuration :type "Float (double-precision)") (TargetCatfish :type "Actor Object Reference"))
  (bind _returnvalue (`self.K2_GetActorLocation` TargetPlayer))
  (`/Engine/EditorBlueprintResources/ActorMacros.Switch Has Authority`
    (:`Authority`
      (bind _outhit (`KismetSystemLibrary.LineTraceSingle` :`Start` _returnvalue :`End` (- _returnvalue (0.0 0.0 3000.0)) :`TraceChannel` "TraceTypeQuery1" :`DrawTime` 10.0))
      (`self.MulticastActivateCatfishVisuals` (`.Location` (`GameplayStatics.BreakHitResult` _outhit)) (`KismetMathLibrary.MakeRotator` 0.0 0.0 (* 360 (`KismetMathLibrary.RandomFloat`))) (0.0 0.0 0.0) TargetCatfish))))

(event `self.Box.OnComponentBeginOverlap`
  (params (OverlappedComponent :type "PrimitiveComponent Object Reference") (OtherActor :type "Actor Object Reference") (OtherComp :type "PrimitiveComponent Object Reference") (OtherBodyIndex :type Integer) (bFromSweep :type Boolean) (SweepResult :type "HitResult Structure (by ref)"))
  (`/Engine/EditorBlueprintResources/ActorMacros.Switch Has Authority`
    (:`Authority`
      (bind _asbp_player (cast `/Game/Blueprints/BP_Player` OtherActor))
      (if (and (!= (stale `Activate` TargetPlayer) OtherActor) (`self.Active`))
        (`|ExecutionSequence`
          (:`then_0`
            (if (not (`/Game/Blueprints/BP_Player.Immune` _asbp_player))
              (set `StolenmatesPlayer.catfished` true _asbp_player)
              (`StolenmatesPlayer.StunPlayer` _asbp_player (stale `Activate` StunDuration))))
          (:`then_1`
            (`self.K2_DestroyActor`)))))))

(fn `UserConstructionScript`)