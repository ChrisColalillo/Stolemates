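; Mystery box pickup that gives an overlapping BP_Player a random power-up.
; A timeline started on BeginPlay spins and bobs the box through its root component.
; On overlap, only the server rolls from the PowerUps array, and if the player holds none, it assigns the pick, decrements the PowerUp_Manager's clamped box count and destroys the box.
; A leftover movement-speed debug snippet is disconnected.
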(event `self.ReceiveBeginPlay`
  (bind _defaultsceneroot (`self.DefaultSceneRoot`))
  ;[1 1 1] Spin and Bob
  (`|ExecutionSequence`
    (:`then_0`
      (set `self.#ofPowerUps` (- (`KismetArrayLibrary.Array_Length` (`self.PowerUps`)) 1))
      (bind _returnvalue (`GameplayStatics.GetActorOfClass` "/Game/Blueprints/PowerUps/PowerUp_Manager.PowerUp_Manager_C"))
      (set `self.PUManager` _returnvalue))
    (:`then_1`
      (bind (_direction _rotation _bob) (`Timeline|Rotate & Bob`)
        (:`Update`
          (`|ExecutionSequence`
            (:`then_0`
              (`/Engine/EditorBlueprintResources/StandardMacros.IsValid` _defaultsceneroot
                (:`Is Valid`
                  (`SceneComponent.K2_SetRelativeRotation` _defaultsceneroot (`KismetMathLibrary.MakeRotator` 0.0 0.0 _rotation) false false))))
            (:`then_1`
              (`/Engine/EditorBlueprintResources/StandardMacros.IsValid` _defaultsceneroot
                (:`Is Valid`
                  (`SceneComponent.K2_SetRelativeLocation` _defaultsceneroot (`KismetMathLibrary.MakeVector` 0.0 0.0 _bob) false false))))))))))

(event `self.ReceiveActorBeginOverlap`
  (params (OtherActor :type "Actor Object Reference"))
  (bind _pumanager (`self.PUManager`))
  ;[1 1 1] Give Player a Random PowerUp
  (`/Engine/EditorBlueprintResources/ActorMacros.Switch Has Authority`
    (:`Authority`
      (bind _asbp_player (cast `/Game/Blueprints/BP_Player` OtherActor))
      (bind _output_get (set `self.PowerUp` (`KismetMathLibrary.RandomIntegerInRange` 0 (`self.#ofPowerUps`))))
      (`KismetSystemLibrary.PrintString` (`KismetStringLibrary.Concat_StrStr` "SERVER MysteryBox picked up | PlayerIndex:" (`KismetStringLibrary.Conv_IntToString` (`StolenmatesPlayer.PlayerIndex` _asbp_player)) "| PowerUp#:" (`KismetStringLibrary.Conv_IntToString` _output_get)))
      (if (not (`/Game/Blueprints/BP_Player.HoldingPU?` _asbp_player))
        (`|ExecutionSequence`
          (:`then_0`
            (`/Game/Blueprints/BP_Player.SetPowerUp` _asbp_player (`|GetArrayItem` (`self.PowerUps`) _output_get) _output_get))
          (:`then_1`
            (set `/Game/Blueprints/PowerUps/PowerUp_Manager.#ofBoxes` (`KismetMathLibrary.Clamp` (- (`/Game/Blueprints/PowerUps/PowerUp_Manager.#ofBoxes` _pumanager) 1) 0 6) _pumanager))
          (:`then_2`
            (`self.K2_DestroyActor`)))))))

(fn `UserConstructionScript`)