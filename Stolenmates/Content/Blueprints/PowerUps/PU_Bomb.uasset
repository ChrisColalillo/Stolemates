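; Bomb power-up projectile that homes in on the nearest player and stuns on impact.
; Activate picks the closest non-owner player within homing range, sets its mesh as the homing target, then starts projectile movement.
; Authority-only overlaps stun non-immune players or detonate on other actors, ignoring the owner and passing through immune players.
; Detonation hides the mesh, plays particles and enables a sphere that stuns players in the blast before delayed destruction.
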(event `Activate`
  (params (OwningPlayer :type "/Game/Blueprints/BP_Player Object Reference") (StunDuration :type "Float (double-precision)") (`Homing Range` :type "Float (double-precision)"))
  (bind _projectilemovement (`self.ProjectileMovement`))
  (`|ExecutionSequence`
    (:`then_0`
      (bind _outactors (`GameplayStatics.GetAllActorsOfClass` "/Game/Blueprints/BP_Player.BP_Player_C"))
      (set `self.ShortestDistance` `Homing Range`))
    (:`then_1`
      (bind _nearestplayer (`self.FindNearestPlayer` _outactors OwningPlayer `Homing Range`))
      (set `ProjectileMovementComponent.HomingTargetComponent` (`Character.Mesh` _nearestplayer) _projectilemovement))
    (:`then_2`
      (`ActorComponent.Activate` _projectilemovement false))
    (:`then_3`
      (set `self.Active` true))))

(event `self.StaticMesh.OnComponentBeginOverlap`
  (params (OverlappedComponent :type "PrimitiveComponent Object Reference") (OtherActor :type "Actor Object Reference") (OtherComp :type "PrimitiveComponent Object Reference") (OtherBodyIndex :type Integer) (bFromSweep :type Boolean) (SweepResult :type "HitResult Structure (by ref)"))
  (`/Engine/EditorBlueprintResources/ActorMacros.Switch Has Authority`
    (:`Authority`
      (bind _asbp_player (cast `/Game/Blueprints/BP_Player` OtherActor)
        (:`then`
          (bind _returnvalue (and (!= (stale `Activate` OwningPlayer) OtherActor) (`self.Active`)))
          (if _returnvalue
            (if (not (`/Game/Blueprints/BP_Player.Immune` _asbp_player))
              (`StolenmatesPlayer.StunPlayer` _asbp_player (stale `Activate` StunDuration))
              (`self.MulticastBombExplodeVisuals` :!label _label)
              (`KismetSystemLibrary.Delay` 1.0)
              (`self.K2_DestroyActor`))))
        (:`CastFailed`
          (if _returnvalue
            (goto _label)))))))

(event `self.Sphere.OnComponentBeginOverlap`
  (params (OverlappedComponent :type "PrimitiveComponent Object Reference") (OtherActor :type "Actor Object Reference") (OtherComp :type "PrimitiveComponent Object Reference") (OtherBodyIndex :type Integer) (bFromSweep :type Boolean) (SweepResult :type "HitResult Structure (by ref)"))
  (`/Engine/EditorBlueprintResources/ActorMacros.Switch Has Authority`
    (:`Authority`
      (bind _asbp_player (cast `/Game/Blueprints/BP_Player` OtherActor))
      (if (and (!= (stale `Activate` OwningPlayer) OtherActor) (`KismetSystemLibrary.IsValid` self))
        (if (not (`/Game/Blueprints/BP_Player.Immune` _asbp_player))
          (`StolenmatesPlayer.StunPlayer` _asbp_player (stale `Activate` StunDuration)))))))

(event `MulticastBombExplodeVisuals`
  (bind _staticmesh (`self.StaticMesh`))
  (`ActorComponent.Deactivate` (`self.ProjectileMovement`))
  (`SceneComponent.SetVisibility` _staticmesh false false)
  (`PrimitiveComponent.SetCollisionEnabled` _staticmesh "NoCollision")
  (`ActorComponent.Activate` (`self.ParticleSystem`) false)
  (`PrimitiveComponent.SetCollisionEnabled` (`self.Sphere`) "QueryOnly"))

(event `CustomEvent`)

(fn `FindNearestPlayer`
  (params (Array :type "Array of /Game/Blueprints/BP_Player Object Reference") (OwningPlayer :type "Object Object Reference") (`Homing Range` :type "Float (double-precision)"))
  (returns (NearestPlayer :type "/Game/Blueprints/BP_Player Object Reference"))
  (for _array_element Array
    (if (!= _array_element OwningPlayer)
      (bind _returnvalue (`self.GetDistanceTo` _array_element))
      (if (< _returnvalue (`self.ShortestDistance`))
        (set `self.ShortestDistance` _returnvalue)
        (set `self.NearestPlayer` _array_element))))
  (return (`self.NearestPlayer`)))

(fn `UserConstructionScript`)