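; PU_Sliding is a power-up actor that makes the activating player's opponents slide for a set duration.
; Activate calls StartSliding on every other non-immune BP_Player with a ground friction multiplier, then waits out the duration.
; It then calls StartSliding with the inverse multiplier and Stop set on all other players, without rechecking immunity, and destroys itself.
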(event `Activate`
  (params (TargetPlayer :type "/Game/Blueprints/BP_Player Object Reference") (Duration :type "Float (double-precision)") (`Sliding Multipler` :type "Float (double-precision)"))
  (bind _outactors (`GameplayStatics.GetAllActorsOfClass` "/Game/Blueprints/BP_Player.BP_Player_C"))
  (for _array_element _outactors
    (if (and (!= _array_element TargetPlayer) (not (`/Game/Blueprints/BP_Player.Immune` _array_element)))
      (`/Game/Blueprints/BP_Player.StartSliding` _array_element `Sliding Multipler` false)))
  (`KismetSystemLibrary.Delay` Duration)
  (for _array_element_2 _outactors
    (if (!= _array_element_2 TargetPlayer)
      (`/Game/Blueprints/BP_Player.StartSliding` _array_element_2 (/ 1.0 `Sliding Multipler`) true)))
  (`self.K2_DestroyActor`))

(fn `UserConstructionScript`)