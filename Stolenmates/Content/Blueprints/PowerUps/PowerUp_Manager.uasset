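; PowerUp_Manager is a Blueprint that activates a player's held power-up: speed boost, sliding, bomb, catfish, mini or immunity.
; ActivateHeldPowerUp switches on the power-up type, casts the supplied object to the matching PU_ class and calls its Activate with the parent player.
; Tuning values such as durations, multipliers, stun times and homing range are hardcoded at each call, and a failed cast does nothing.
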(event `ActivateHeldPowerUp`
  (params (PowerUp :type "Object Object Reference") (ParentPlayer :type "/Game/Blueprints/BP_Player Object Reference") (`PowerUp#` :type Integer))
  ;[1 1 1] PowerUp Variables
  (switch `int` `PowerUp#`
    (:`0`
      (bind _aspu_speed_boost (cast `/Game/Blueprints/PowerUps/PU_SpeedBoost` PowerUp))
      (`/Game/Blueprints/PowerUps/PU_SpeedBoost.Activate` _aspu_speed_boost ParentPlayer 5.0 1.5))
    (:`1`
      (bind _aspu_sliding (cast `/Game/Blueprints/PowerUps/PU_Sliding` PowerUp))
      (`/Game/Blueprints/PowerUps/PU_Sliding.Activate` _aspu_sliding ParentPlayer 8.0 4.0))
    (:`2`
      (bind _aspu_bomb (cast `/Game/Blueprints/PowerUps/PU_Bomb` PowerUp))
      (`/Game/Blueprints/PowerUps/PU_Bomb.Activate` _aspu_bomb ParentPlayer 1.5 10000.0))
    (:`3`
      (bind _aspu_catfish (cast `/Game/Blueprints/PowerUps/PU_Catfish` PowerUp))
      (`/Game/Blueprints/PowerUps/PU_Catfish.Activate` _aspu_catfish ParentPlayer 3.0 _aspu_catfish))
    (:`4`
      (bind _aspu_mini (cast `/Game/Blueprints/PowerUps/PU_Mini` PowerUp))
      (`/Game/Blueprints/PowerUps/PU_Mini.Activate` _aspu_mini ParentPlayer 5.0 0.5))
    (:`5`
      (bind _aspu_immunity (cast `/Game/Blueprints/PowerUps/PU_Immunity` PowerUp))
      (`/Game/Blueprints/PowerUps/PU_Immunity.Activate` _aspu_immunity ParentPlayer 7.0))))

(fn `UserConstructionScript`)