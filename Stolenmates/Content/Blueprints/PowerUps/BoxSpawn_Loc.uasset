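; Mystery box spawn point for power-ups, which places a MysteryBox at its location through a ChildActor component.
; On BeginPlay, only the authority caches the PowerUp_Manager and starts an endless random-delay polling loop.
; When the child slot is empty, it sets the child class to spawn a box and increments the manager's shared count, provided that count is below the hardcoded cap of six.
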(event `self.ReceiveBeginPlay`
  (bind _pumanager (`self.PUManager`))
  (bind _returnvalue (`KismetMathLibrary.RandomFloatInRange` (`self.SpawnTimeMin`) (`self.SpawnTimeMax`)))
  (bind __ofboxes (`/Game/Blueprints/PowerUps/PowerUp_Manager.#ofBoxes` _pumanager))
  (`/Engine/EditorBlueprintResources/ActorMacros.Switch Has Authority`
    (:`Authority`
      (`|ExecutionSequence`
        (:`then_0`
          (`/Engine/EditorBlueprintResources/StandardMacros.DoOnce` false
            (:`Completed`
              (bind _returnvalue_2 (`GameplayStatics.GetActorOfClass` "/Game/Blueprints/PowerUps/PowerUp_Manager.PowerUp_Manager_C"))
              (set `self.PUManager` _returnvalue_2))))
        (:`then_1`
          (`/Engine/EditorBlueprintResources/StandardMacros.IsValid` (`SceneComponent.GetChildComponent` (`self.ChildActor`) 0) :!label _label
            (:`Is Valid`
              (`KismetSystemLibrary.Delay` _returnvalue)
              (goto _label))
            (:`Is Not Valid`
              (`KismetSystemLibrary.Delay` _returnvalue)
              (if (< __ofboxes 6)
                (`ChildActorComponent.SetChildActorClass` (`self.ChildActor`) "/Game/Blueprints/PowerUps/MysteryBox.MysteryBox_C")
                (`KismetSystemLibrary.PrintString` (`KismetStringLibrary.Concat_StrStr` "SERVER spawned MysteryBox from" (`KismetSystemLibrary.GetDisplayName` self) "at " (`KismetStringLibrary.Conv_VectorToString` (`self.K2_GetActorLocation`))))
                (set `/Game/Blueprints/PowerUps/PowerUp_Manager.#ofBoxes` (+ __ofboxes 1) _pumanager)
                (goto _label)
                (else
                  (goto _label))))))))))

(fn `UserConstructionScript`)