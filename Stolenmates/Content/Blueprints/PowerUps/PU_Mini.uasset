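; Mini power-up actor that temporarily shrinks the activating player's opponents.
; Activate applies the mini state at a given scale to every BP_Player except the target, skipping immune or already-mini players, with multicast shrink VFX.
; After the duration it restores any mini player from the same list, regardless of which power-up shrank them, then destroys itself.
; The restore pass switches the shrink VFX on twice and never off.
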(event `Activate`
  (params (TargetPlayer :type "/Game/Blueprints/BP_Player Object Reference") (Duration :type "Float (double-precision)") (`Scale Multipler` :type "Float (double-precision)"))
  (bind _outactors (`GameplayStatics.GetAllActorsOfClass` "/Game/Blueprints/BP_Player.BP_Player_C"))
  (for _array_element _outactors
    (if (and (!= _array_element TargetPlayer) (not (`/Game/Blueprints/BP_Player.Immune` _array_element)) (not (`StolenmatesPlayer.Mini` _array_element)))
      (bind _shrink (`/Game/Blueprints/BP_Player.Shrink` _array_element))
      (`/Game/Blueprints/BP_Player.MulticastSetPlayerVFX` _array_element _shrink true)
      (`/Game/Blueprints/BP_Player.ApplyMiniState` _array_element true `Scale Multipler`)
      (`/Game/Blueprints/BP_Player.MulticastSetPlayerVFX` _array_element _shrink false)))
  ;[1 1 1] Destroy and reverse effects after PU_Mini ends
  (`KismetSystemLibrary.Delay` Duration)
  (for _array_element_2 _outactors
    (if (`StolenmatesPlayer.Mini` _array_element_2)
      (bind _shrink_2 (`/Game/Blueprints/BP_Player.Shrink` _array_element_2))
      (`/Game/Blueprints/BP_Player.MulticastSetPlayerVFX` _array_element_2 _shrink_2 true)
      (`/Game/Blueprints/BP_Player.ApplyMiniState` _array_element_2 false `Scale Multipler`)
      (`/Game/Blueprints/BP_Player.MulticastSetPlayerVFX` _array_element_2 _shrink_2 true)))
  (`self.K2_DestroyActor`))

(fn `UserConstructionScript`)