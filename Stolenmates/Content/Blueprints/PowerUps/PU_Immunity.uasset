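; Immunity power-up that makes the target player immune for a given duration.
; On Activate it sets the player's Immune flag and multicasts the heart and spark shield VFX on.
; After a delay it clears the flag, switches both effects off and destroys itself.
; The construction script only calls its parent.
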(event `Activate`
  (params (TargetPlayer :type "/Game/Blueprints/BP_Player Object Reference") (Duration :type "Float (double-precision)"))
  (bind _heartshield (`/Game/Blueprints/BP_Player.HeartShield` TargetPlayer))
  (bind _sparkshield (`/Game/Blueprints/BP_Player.SparkShield` TargetPlayer))
  (`|ExecutionSequence`
    (:`then_0`
      (set `/Game/Blueprints/BP_Player.Immune` true TargetPlayer)
      (`/Game/Blueprints/BP_Player.MulticastSetPlayerVFX` TargetPlayer _heartshield true)
      (`/Game/Blueprints/BP_Player.MulticastSetPlayerVFX` TargetPlayer _sparkshield true))
    (:`then_1`
      (`KismetSystemLibrary.Delay` Duration)
      (set `/Game/Blueprints/BP_Player.Immune` false TargetPlayer)
      (`/Game/Blueprints/BP_Player.MulticastSetPlayerVFX` TargetPlayer _heartshield false)
      (`/Game/Blueprints/BP_Player.MulticastSetPlayerVFX` TargetPlayer _sparkshield false)
      (`self.K2_DestroyActor`))))

(fn `UserConstructionScript`
  (`parent.UserConstructionScript`))