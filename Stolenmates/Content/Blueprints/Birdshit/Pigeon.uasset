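; Pigeon character that fades in on spawn, wanders between random points and can fly away and despawn.
; BeginPlay fills PatrolPoints with navigable locations near its start, then Patrol cycles through them with AI MoveTo, re-calling itself on success.
; FlyAway changes walk speed, jumps after a short delay and fades out, destroying the actor.
; Both fades share one timeline, played forward or reversed on a dynamic material, with the normal material restored after fade-in.
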(event `self.ReceiveBeginPlay`
  (bind _patrolpoints (`self.PatrolPoints`))
  ;[1 1 1] Fade in and set random patrol points
  (`|ExecutionSequence`
    (:`then_0`
      (`self.FadeMaterial` true))
    (:`then_1`
      (for (_ _array_index) _patrolpoints
        (bind _randomlocation (`NavigationSystemV1.K2_GetRandomLocationInNavigableRadius` (`self.K2_GetActorLocation`) 150.0 null null))
        (`KismetArrayLibrary.Array_Set` _patrolpoints _array_index _randomlocation))
      (`self.Patrol`))))

(event `Patrol`
  (bind _nextpoint (`self.NextPoint`))
  ;[1 1 1] Patrol
  (`|AIMoveTo` self (`|GetArrayItem` (`self.PatrolPoints`) (`self.NextPoint`)) null 10.0
    (:`OnSuccess`
      (if (>= _nextpoint (- (`KismetArrayLibrary.Array_Length` (`self.PatrolPoints`)) 1))
        (set `self.NextPoint` 0)
        (else
          (set `self.NextPoint` (+ _nextpoint 1))))
      (`self.Patrol`))))

(event `FadeMaterial`
  (params (`FadeIn?` :type Boolean))
  ;[1 1 1] Fade in or out
  (`/Engine/EditorBlueprintResources/StandardMacros.DoOnce` false :!label _label
    (:`Completed`
      (bind _returnvalue (`PrimitiveComponent.CreateDynamicMaterialInstance` (`self.Mesh`) 0 "/Game/Art/Materials/Textures/PigeonInvis.PigeonInvis" "None"))
      (if `FadeIn?`
        (`MaterialInstanceDynamic.SetScalarParameterValue` _returnvalue "FadeOut" 0.0)
        (bind (_direction _fade) (`Timeline|Fade` :!via `PlayFromStart` :!label _label_2)
          (:`Update`
            (`MaterialInstanceDynamic.SetScalarParameterValue` _returnvalue "FadeOut" _fade))
          (:`Finished`
            (if `FadeIn?`
              (`PrimitiveComponent.SetMaterial` (`self.Mesh`) 0 "/Game/Art/Materials/Textures/Pigeon.Pigeon")
              (goto _label :!via `Reset`)
              (else
                (`self.K2_DestroyActor`)))))
        (else
          (`MaterialInstanceDynamic.SetScalarParameterValue` _returnvalue "FadeOut" 1.0)
          (goto _label_2 :!via `ReverseFromEnd`))))))

(event `Fly Away`
  ;[1 1 1] Fly away
  (set `self.FlyAway` true)
  (set `CharacterMovementComponent.MaxWalkSpeed` 200.0 (`self.CharacterMovement`))
  (`KismetSystemLibrary.Delay` 0.3)
  (`self.Jump`)
  (`self.FadeMaterial` false))

(fn `UserConstructionScript`)