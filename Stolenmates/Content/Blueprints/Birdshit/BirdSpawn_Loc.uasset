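; Pigeon spawn point that leaves a temporary poop slow zone when a player scares the flock away.
; The server spawns pigeons at set offsets while fewer than four flocks are counted in PowerUp_Manager, otherwise retrying after a random delay.
; Entering ScareArea despawns the flock, schedules a respawn and multicasts a timeline fade toggling SlowArea collision.
; SlowArea slows non-immune players and blocks jumping until they leave.
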(event `self.ReceiveBeginPlay`
  ;[1 1 1] Spawn Pigeons and ignore slow area
  (`/Engine/EditorBlueprintResources/ActorMacros.Switch Has Authority`
    (:`Authority`
      (`PrimitiveComponent.SetCollisionResponseToAllChannels` (`self.SlowArea`) "ECR_Ignore")
      (bind _returnvalue (`GameplayStatics.GetActorOfClass` "/Game/Blueprints/PowerUps/PowerUp_Manager.PowerUp_Manager_C"))
      (set `self.PUManager` _returnvalue)
      (`self.Spawn Pigeons`))))

(event `Spawn Pigeons`
  (bind _pumanager (`self.PUManager`))
  (bind __ofpigeons (`/Game/Blueprints/PowerUps/PowerUp_Manager.#ofPigeons` _pumanager))
  ;[1 1 1] Spawn Pigeons
  (if (< __ofpigeons 4) :!label _label
    (for (_array_element _array_index) (`self.Pigeon Spawns`)
      (bind _returnvalue (`|SpawnActorFromClass` "/Game/Blueprints/Birdshit/Pigeon.Pigeon_C" (`KismetMathLibrary.MakeTransform` (+ _array_element (`self.K2_GetActorLocation`))) "AdjustIfPossibleButAlwaysSpawn" "OverrideRootScale" null null))
      (`KismetArrayLibrary.Array_Set` (`self.Pigeons`) _array_index _returnvalue))
    (set `/Game/Blueprints/PowerUps/PowerUp_Manager.#ofPigeons` (+ __ofpigeons 1) _pumanager)
    (set `self.Active` true)
    (else
      (`KismetSystemLibrary.Delay` (`KismetMathLibrary.RandomFloatInRange` (`self.SpawnTimeMin`) (`self.SpawnTimeMax`)))
      (goto _label))))

(event `self.Scare Area.OnComponentBeginOverlap`
  (params (OverlappedComponent :type "PrimitiveComponent Object Reference") (OtherActor :type "Actor Object Reference") (OtherComp :type "PrimitiveComponent Object Reference") (OtherBodyIndex :type Integer) (bFromSweep :type Boolean) (SweepResult :type "HitResult Structure (by ref)"))
  ;[1 1 1] Cause pigeons to fly away and enable slow area
  (`/Engine/EditorBlueprintResources/ActorMacros.Switch Has Authority`
    (:`Authority`
      (cast `/Game/Blueprints/BP_Player` OtherActor)
      (if (`self.Active`)
        (`/Engine/EditorBlueprintResources/StandardMacros.DoOnce` false :!label _label_2
          (:`Completed`
            (`|ExecutionSequence`
              (:`then_0`
                (`self.Despawn Pigeons`))
              (:`then_1`
                (`self.MulticastSetSlowArea` true))
              (:`then_2`
                (`KismetSystemLibrary.Delay` (`self.TimePoopLasts`))
                (`self.MulticastSetSlowArea` false)))))))))

(event `Despawn Pigeons`
  (bind _pumanager (`self.PUManager`))
  ;[1 1 1] Despawn Pigeons
  (for _array_element (`self.Pigeons`)
    (`/Engine/EditorBlueprintResources/StandardMacros.IsValid` _array_element
      (:`Is Valid`
        (`/Game/Blueprints/Birdshit/Pigeon.Fly Away` _array_element))))
  (set `/Game/Blueprints/PowerUps/PowerUp_Manager.#ofPigeons` (- (`/Game/Blueprints/PowerUps/PowerUp_Manager.#ofPigeons` _pumanager) 1) _pumanager)
  (set `self.Active` false)
  (`KismetSystemLibrary.Delay` (`KismetMathLibrary.RandomFloatInRange` (`self.SpawnTimeMin`) (`self.SpawnTimeMax`)))
  (`self.Spawn Pigeons`)
  (goto _label_2 :!via `Reset`))

(event `self.SlowArea.OnComponentBeginOverlap`
  (params (OverlappedComponent :type "PrimitiveComponent Object Reference") (OtherActor :type "Actor Object Reference") (OtherComp :type "PrimitiveComponent Object Reference") (OtherBodyIndex :type Integer) (bFromSweep :type Boolean) (SweepResult :type "HitResult Structure (by ref)"))
  ;[1 1 1] Slow and ground player
  (bind _asbp_player (cast `/Game/Blueprints/BP_Player` OtherActor))
  (if (not (`/Game/Blueprints/BP_Player.Immune` _asbp_player))
    (bind _charactermovement (`Character.CharacterMovement` _asbp_player))
    (set `CharacterMovementComponent.JumpZVelocity` 0.0 _charactermovement)
    (set `CharacterMovementComponent.MaxWalkSpeed` (* (`CharacterMovementComponent.MaxWalkSpeed` _charactermovement) (`self.Slow Multiplier`)) _charactermovement)))

(event `FadeMaterial`
  (params (`FadeIn?` :type Boolean))
  (bind _slowarea (`self.SlowArea`))
  ;[1 1 1] Fade in or out
  (bind _returnvalue (`PrimitiveComponent.CreateDynamicMaterialInstance` (`self.SlowArea`) 0 "/Game/Art/Materials/Textures/BirdPoopInvis.BirdPoopInvis" "None"))
  (if `FadeIn?`
    (`MaterialInstanceDynamic.SetScalarParameterValue` _returnvalue "FadeOut" 0.0)
    (bind (_direction _fade) (`Timeline|Fade` :!via `PlayFromStart` :!label _label_3)
      (:`Update`
        (`MaterialInstanceDynamic.SetScalarParameterValue` _returnvalue "FadeOut" _fade))
      (:`Finished`
        (if `FadeIn?`
          (`PrimitiveComponent.SetCollisionResponseToAllChannels` _slowarea "ECR_Overlap")
          (else
            (`PrimitiveComponent.SetCollisionResponseToAllChannels` _slowarea "ECR_Ignore")))))
    (else
      (`MaterialInstanceDynamic.SetScalarParameterValue` _returnvalue "FadeOut" 1.0)
      (goto _label_3 :!via `ReverseFromEnd`))))

(event `self.SlowArea.OnComponentEndOverlap`
  (params (OverlappedComponent :type "PrimitiveComponent Object Reference") (OtherActor :type "Actor Object Reference") (OtherComp :type "PrimitiveComponent Object Reference") (OtherBodyIndex :type Integer))
  ;[1 1 1] Slow and ground player
  (bind _asbp_player (cast `/Game/Blueprints/BP_Player` OtherActor))
  (bind _charactermovement (`Character.CharacterMovement` _asbp_player))
  (set `CharacterMovementComponent.JumpZVelocity` 1000.0 _charactermovement)
  (bind _maxwalkspeed (`CharacterMovementComponent.MaxWalkSpeed` _charactermovement))
  (if (< _maxwalkspeed 1000.0)
    (set `CharacterMovementComponent.MaxWalkSpeed` (/ _maxwalkspeed (`self.Slow Multiplier`)) _charactermovement)))

(event `MulticastSetSlowArea`
  (params (bActive :type Boolean))
  (if bActive
    (`self.FadeMaterial` true)
    (else
      (`self.FadeMaterial` false))))

(fn `UserConstructionScript`)