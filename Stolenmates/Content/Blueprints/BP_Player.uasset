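; Player character Blueprint for Stolemates that carries and uses power-ups, receives their effects and wears per-index materials and decals.
; Held power-ups attach to the hand, activate through PowerUp_Manager and update the HUD via the game mode.
; Effect events handle timed speed boosts with multicast trail VFX, roller-blade sliding and mini scaling.
; Steam and standard inputs share ability and pause logic, branching on MatchType between local handling and online requests.
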(event `self.SteamInputUseAbilityPressed_BP`
  (bind _heldpowerup (`self.HeldPowerUp`))
  (if (not (`self.bInputLocked`)) :!label _label
    (bind _asstolemates_game_instance (cast `StolematesGameInstance` (`GameplayStatics.GetGameInstance`)))
    (switch `EMatchType` (`StolematesGameInstance.MatchType` _asstolemates_game_instance)
      (:`Local`
        ;[1 1 1] Activate PowerUp
        (`/Engine/EditorBlueprintResources/StandardMacros.IsValid` _heldpowerup :!label _label_2
          (:`Is Valid`
            (`|ExecutionSequence`
              (:`then_0`
                (`self.K2_DetachFromActor` _heldpowerup "KeepWorld" "KeepWorld" "KeepWorld")
                (`/Game/Blueprints/PowerUps/PowerUp_Manager.ActivateHeldPowerUp` (`self.PU_Manager`) _heldpowerup self (`self.PowerUp#`)))
              (:`then_1`
                (set `self.HoldingPU?` false)
                (set `self.HeldPowerUp` null))
              (:`then_2`
                (bind _asstolenmates_game_mode_base (cast `StolenmatesGameModeBase` (`GameplayStatics.GetGameMode`)))
                (`StolenmatesGameModeBase.BroadcastPowerUpHUDUpdate` _asstolenmates_game_mode_base (`self.PlayerIndex`) 6))))))
      (:`Online`
        (`self.Server_UsePowerUp`)))))

(event `InputAction|UseAbility`
  (params (Key :type "Key Structure"))
  (:`Pressed`
    (goto _label)))

(event `self.ReceiveBeginPlay`
  (`|ExecutionSequence`
    (:`then_0`
      (bind _returnvalue (`GameplayStatics.GetActorOfClass` "/Game/Blueprints/PowerUps/PowerUp_Manager.PowerUp_Manager_C"))
      (set `self.PU_Manager` _returnvalue))
    (:`then_1`
      (bind _asbp_game_mode (cast `/Game/Blueprints/BP_GameMode` (`GameplayStatics.GetGameMode`)))
      (set `self.GameMode` _asbp_game_mode))
    (:`then_2`
      (`KismetSystemLibrary.Delay` 0.2)
      (`self.ApplyPlayerVisuals`))))

(event `Server_UsePowerUp`
  ;[1 1 1] Activate PowerUp
  (if (not (`self.bInputLocked`))
    (goto _label_2)))

(event `MulticastSetPlayerVFX`
  (params (Particle :type "ParticleSystemComponent Object Reference") (bActive :type Boolean))
  (if bActive
    (`ActorComponent.Activate` Particle false)
    (else
      (`ActorComponent.Deactivate` Particle))))

(event `SetPowerUp`
  (params (PowerUpType :type "Actor Class Reference (by ref)") (`PowerUp#` :type Integer))
  (bind _mesh (`self.Mesh`))
  ;[1 1 1] Sets the Player's PowerUp
  (`|ExecutionSequence`
    (:`then_0`
      (bind _returnvalue (`|SpawnActorFromClass` PowerUpType (`KismetMathLibrary.MakeTransform` (`SceneComponent.GetSocketLocation` _mesh "RightHand2_JNTSocket")) "Undefined" "OverrideRootScale" null null))
      (set `self.HeldPowerUp` _returnvalue))
    (:`then_1`
      (`self.K2_AttachToComponent` _returnvalue _mesh "RightHand2_JNTSocket" "KeepWorld" "KeepWorld" "KeepWorld" true))
    (:`then_2`
      (set `self.PowerUp#` `PowerUp#`)
      (set `self.HoldingPU?` true))
    (:`then_3`
      (bind _asstolenmates_game_mode_base (cast `StolenmatesGameModeBase` (`GameplayStatics.GetGameMode`)))
      (`StolenmatesGameModeBase.BroadcastPowerUpHUDUpdate` _asstolenmates_game_mode_base (`self.PlayerIndex`) `PowerUp#`))))

(event `SpeedPlayer`
  (params (Duration :type "Float (double-precision)") (SpeedMultiplier :type "Float (double-precision)"))
  (bind _charactermovement (`self.CharacterMovement`))
  (bind _trail (`self.Trail`))
  (bind _maxwalkspeed (`CharacterMovementComponent.MaxWalkSpeed` _charactermovement))
  ;[1 1 1] Call for a SpeedBoost
  (`/Engine/EditorBlueprintResources/StandardMacros.DoOnce` false :!label _label_3
    (:`Completed`
      (set `CharacterMovementComponent.MaxWalkSpeed` (* _maxwalkspeed SpeedMultiplier) _charactermovement)
      (`self.MulticastSetPlayerVFX` _trail true)
      (`KismetSystemLibrary.Delay` Duration)
      (set `CharacterMovementComponent.MaxWalkSpeed` (/ _maxwalkspeed SpeedMultiplier) _charactermovement)
      (`self.MulticastSetPlayerVFX` _trail)
      (goto _label_3 :!via `Reset`))))

(event `StartSliding`
  (params (GroundFrictionMultiplier :type "Float (double-precision)") (Stop :type Boolean))
  (bind _returnvalue (`self.GetActorScale3D`))
  (bind _mesh (`self.Mesh`))
  (bind _charactermovement (`self.CharacterMovement`))
  (bind (_returnvalue_roll _returnvalue_pitch _returnvalue_yaw) (`KismetMathLibrary.BreakRotator` (`SceneComponent.K2_GetComponentRotation` _mesh)))
  (bind _returnvalue_2 (/ (`CharacterMovementComponent.GroundFriction` _charactermovement) GroundFrictionMultiplier))
  ;[1 1 1] Start Sliding
  (if Stop
    (set `CharacterMovementComponent.GroundFriction` _returnvalue_2 _charactermovement)
    (set `CharacterMovementComponent.MaxAcceleration` 8192.0 _charactermovement)
    (`|ExecutionSequence`
      (:`then_0`
        (`/Engine/EditorBlueprintResources/StandardMacros.IsValid` (stale _returnvalue_3)
          (:`Is Valid`
            (`self.K2_DestroyActor` (stale _returnvalue_3)))))
      (:`then_1`
        (`/Engine/EditorBlueprintResources/StandardMacros.IsValid` (stale _returnvalue_4)
          (:`Is Valid`
            (`self.K2_DestroyActor` (stale _returnvalue_4)))))
      (:`then_2`
        (goto _label_4 :!via `Reset`)))
    (else
      (`/Engine/EditorBlueprintResources/StandardMacros.DoOnce` false :!label _label_4
        (:`Completed`
          (`|ExecutionSequence`
            (:`then_0`
              (set `CharacterMovementComponent.MaxAcceleration` 2048.0 _charactermovement)
              (set `CharacterMovementComponent.GroundFriction` _returnvalue_2 _charactermovement))
            (:`then_1`
              (`|ExecutionSequence`
                (:`then_0`
                  (bind _returnvalue_3 (`|SpawnActorFromClass` "/Game/Blueprints/PowerUps/RollerBlades.RollerBlades_C" (`KismetMathLibrary.MakeTransform` (`SceneComponent.GetSocketLocation` _mesh "RightFoot_JNTSocket") (`KismetMathLibrary.MakeRotator` 0.0 0.0 _returnvalue_yaw) _returnvalue) "Undefined" "OverrideRootScale" null null))
                  (`self.K2_AttachToComponent` _returnvalue_3 _mesh "RightFoot_JNTSocket" "KeepWorld" "KeepWorld" "KeepWorld" true))
                (:`then_1`
                  (bind _returnvalue_4 (`|SpawnActorFromClass` "/Game/Blueprints/PowerUps/RollerBlades.RollerBlades_C" (`KismetMathLibrary.MakeTransform` (`SceneComponent.GetSocketLocation` _mesh "LeftFoot_JNTSocket") (`KismetMathLibrary.MakeRotator` 0.0 0.0 _returnvalue_yaw) _returnvalue) "Undefined" "OverrideRootScale" null null))
                  (`self.K2_AttachToComponent` _returnvalue_4 _mesh "LeftFoot_JNTSocket" "KeepWorld" "KeepWorld" "KeepWorld" true))))))))))

(event `self.SteamInputPausePressed_BP`
  (bind _pausemenu (`self.PauseMenu`))
  (bind _returnvalue (`self.GetController` self))
  ;[1 1 1] Pause
  (if (not (`self.gameOver`)) :!label _label_5
    (bind _asstolemates_game_instance (cast `StolematesGameInstance` (`GameplayStatics.GetGameInstance`)))
    (switch `EMatchType` (`StolematesGameInstance.MatchType` _asstolemates_game_instance)
      (:`Local`
        (`/Engine/EditorBlueprintResources/StandardMacros.IsValid` (`self.PauseMenu`)
          (:`Is Valid`
            _)
          (:`Is Not Valid`
            (bind _asplayer_controller (cast `PlayerController` (`self.GetController` self)))
            (bind _returnvalue_2 (`|CreateWidget` "/Game/Blueprints/PauseMenu.PauseMenu_C" _asplayer_controller))
            (set `self.PauseMenu` _returnvalue_2)))
        (if (`GameplayStatics.IsGamePaused`)
          (bind _asplayer_controller_2 (cast `PlayerController` _returnvalue))
          (`Widget.RemoveFromParent` _pausemenu)
          (bind _returnvalue_3 (`GameplayStatics.SetGamePaused` false))
          (set `PlayerController.bShowMouseCursor` _returnvalue_3 _asplayer_controller_2)
          (`WidgetBlueprintLibrary.SetInputMode_GameOnly` _asplayer_controller_2)
          (else
            (bind _asplayer_controller_3 (cast `PlayerController` _returnvalue))
            (`UserWidget.AddToViewport` _pausemenu 0)
            (set `PlayerController.bShowMouseCursor` true _asplayer_controller_3)
            (`WidgetBlueprintLibrary.SetInputMode_GameAndUIEx` _asplayer_controller_3 _pausemenu "DoNotLock" false)
            (`Widget.SetUserFocus` _pausemenu _asplayer_controller_3)
            (`Widget.SetUserFocus` (`/Game/Blueprints/PauseMenu.Resume` _pausemenu) _asplayer_controller_3)
            (`GameplayStatics.SetGamePaused` true))))
      (:`Online`
        (bind _asstolemates_player_controller (cast `StolematesPlayerController` (`GameplayStatics.GetPlayerController` 0)))
        (`StolematesPlayerController.RequestPauseGame` _asstolemates_player_controller)))))

(event `InputAction|Pause` :paused true
  (params (Key :type "Key Structure"))
  ;[1 1 1] Pause
  (:`Pressed`
    (goto _label_5)))

(event `ApplyMiniState`
  (params (IsMini :type Boolean) (ScaleMultiplier :type "Float (double-precision)"))
  (bind _returnvalue (`self.GetActorScale3D`))
  ;[1 1 1] Mini
  (if IsMini
    (set `self.Mini` true)
    (`self.SetActorScale3D` (* _returnvalue ScaleMultiplier))
    (else
      (set `self.Mini` false)
      (`self.SetActorScale3D` (/ _returnvalue ScaleMultiplier)))))

(fn `ApplyPlayerVisuals`
  (bind _playerindex (`self.PlayerIndex`))
  (bind _playermaterials (`self.PlayerMaterials`))
  (if (and (>= _playerindex 0) (< _playerindex (`KismetArrayLibrary.Array_Length` _playermaterials)))
    (`PrimitiveComponent.SetMaterial` (`self.Mesh`) 0 (`|GetArrayItem` _playermaterials _playerindex))
    (`DecalComponent.SetDecalMaterial` (`self.PlayerDecal`) (`|GetArrayItem` (`self.PlayerDecals`) _playerindex))))

(fn `UserConstructionScript`)