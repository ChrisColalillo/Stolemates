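; Player character Blueprint that triggers three power-ups from input: Catfish, Love Bomb and Lovestruck.
; Inputs pass an ID to ActivatePowerup, whose mapping swaps Love Bomb and Lovestruck relative to their input names.
; Catfish and Love Bomb spawn actors at the capsule, the bomb then homing; Lovestruck briefly doubles walk speed.
; Love Bomb and Lovestruck consume availability flags, Fly Me to the Moon is empty, and O toggles HasHeart for testing.
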(event `activate Lovestruck`
  (bind _charactermovement (`self.CharacterMovement`))
  ;[1 1 1] activate LoveStruck
  (if (`self.LoveStruck`)
    (set `CharacterMovementComponent.MaxWalkSpeed` 2400.0 _charactermovement)
    (set `self.LoveStruck` false)
    (`KismetSystemLibrary.Delay` 2.0)
    (set `CharacterMovementComponent.MaxWalkSpeed` 1200.0 _charactermovement)))

(event `Key|O`
  (params (Key :type "Key Structure"))
  ;[1 1 1] made for testing purposes
  (:`Pressed`
    (`/Engine/EditorBlueprintResources/StandardMacros.FlipFlop`
      (:`A`
        (set `self.hasHeart` true)
        (`KismetSystemLibrary.PrintString` "hasheart on"))
      (:`B`
        (set `self.hasHeart` false)
        (`KismetSystemLibrary.PrintString` "hasheart off")))))

(event `InputAction|Catfish`
  (params (Key :type "Key Structure"))
  ;[1 1 1] Activate Power up
  (:`Pressed`
    (if true
      (set `self.temp_power_up` 0)
      (`self.activate powerup` (`self.temp_power_up`) :!label _label)
      (set `self.temp_power_up` (`self.max_powerup`)))))

(event `InputAction|LoveBomb`
  (params (Key :type "Key Structure"))
  ;[1 1 1] Activate Power up
  (:`Pressed`
    (if true
      (set `self.temp_power_up` 1)
      (goto _label))))

(event `InputAction|Lovestruck`
  (params (Key :type "Key Structure"))
  ;[1 1 1] Activate Power up
  (:`Pressed`
    (if true
      (set `self.temp_power_up` 2)
      (goto _label))))

(fn `activate Catfish`
  (`|SpawnActorFromClass` "/Game/Blueprints/Ivans_terrotory/Old_pracrtices/PowerUp_Catfish.PowerUp_Catfish_C" (`KismetMathLibrary.Conv_VectorToTransform` (`SceneComponent.K2_GetComponentLocation` (`self.CapsuleComponent`))) "AlwaysSpawn" "OverrideRootScale" self null)
  (set `self.Catfish` false))

(fn `activate fly me to the moon`)

(fn `activate Love Bomb`
  (if (`self.LoveBomb`)
    (bind _returnvalue (`|SpawnActorFromClass` "/Game/Blueprints/Ivans_terrotory/Old_pracrtices/PowerUp_LoveBomb.PowerUp_LoveBomb_C" (`KismetMathLibrary.MakeTransform` (`SceneComponent.K2_GetComponentLocation` (`self.CapsuleComponent`))) "AdjustIfPossibleButAlwaysSpawn" "OverrideRootScale" self null))
    (set `self.LoveBomb` false)
    (`/Game/Blueprints/Ivans_terrotory/Old_pracrtices/PowerUp_LoveBomb.homing` _returnvalue)))

(fn `activate powerup`
  (params (`power_up ID` :type Integer))
  (`KismetSystemLibrary.PrintString` (`KismetStringLibrary.Conv_IntToString` `power_up ID`))
  (if (== `power_up ID` 0)
    (`self.activate Catfish`)
    (elif (== `power_up ID` 1)
      (`self.activate_Lovestruck`)
      (elif (== `power_up ID` 2)
        (`self.activate Love Bomb`)
        (elif (== `power_up ID` (`self.max_powerup`))
          (`KismetSystemLibrary.PrintString` "no power up found"))))))

(fn `activate_Lovestruck`
  (`self.activate Lovestruck`))

(fn `UserConstructionScript`)