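; BP_CN_Tower_Launch is a launch point that sends the ability user along a spline path.
; Its Box overlap registers it as the player's static ability, and leaving calls SetAbility again without that reference.
; FireAbility spawns a BP_FollowSpline at the actor's transform, passing the spline, total travel time and the user as follower.
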(event `self.fireAbility`
  (params (abilityUser :type "StolenmatesPlayer Object Reference"))
  (`|SpawnActorFromClass` "/Game/Blueprints/BP_FollowSpline.BP_FollowSpline_C" (`self.GetTransform`) "AlwaysSpawn" "OverrideRootScale" null (`self.Spline`) (`self.Total Travel Time`) abilityUser null))

(event `self.Box.OnComponentBeginOverlap`
  (params (OverlappedComponent :type "PrimitiveComponent Object Reference") (OtherActor :type "Actor Object Reference") (OtherComp :type "PrimitiveComponent Object Reference") (OtherBodyIndex :type Integer) (bFromSweep :type Boolean) (SweepResult :type "HitResult Structure (by ref)"))
  (bind _asbp_player (cast `/Game/Blueprints/BP_Player` OtherActor))
  (`StolenmatesPlayer.SetAbility` _asbp_player "ZONE_ABILITY_OVERRIDE" self))

(event `self.Box.OnComponentEndOverlap`
  (params (OverlappedComponent :type "PrimitiveComponent Object Reference") (OtherActor :type "Actor Object Reference") (OtherComp :type "PrimitiveComponent Object Reference") (OtherBodyIndex :type Integer))
  (bind _asbp_player (cast `/Game/Blueprints/BP_Player` OtherActor))
  (`StolenmatesPlayer.SetAbility` _asbp_player "ZONE_ABILITY_OVERRIDE" null))

(fn `UserConstructionScript`)