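; Player controller for Stolemates that owns the match UI: in-game HUD, power-up display, waiting-for-players message, online pause menu and win screen.
; Events create and remove the widgets, caching references, while the HUD and pause events also switch input mode and cursor.
; The win screen branches on the game instance's match type so only the winner's controller shows it locally.
; Showing the waiting message also marks match-start ready, and main-menu returns go through the game instance.
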(event `self.ShowInGameHUD`
  (params (PlayerCount :type Integer) (TimeToWin :type "Float (single-precision)"))
  ;[1 1 1] In-game HUD
  (bind _returnvalue (`|CreateWidget` "/Game/Blueprints/HUD.HUD_C" self))
  (bind _output_get (set `self.HUDRef` _returnvalue))
  (`/Game/Blueprints/HUD.SetHUDPlayerCount` _output_get PlayerCount)
  (set `/Game/Blueprints/HUD.TimeToWin` TimeToWin _output_get)
  (`UserWidget.AddToViewport` _output_get 0)
  (`WidgetBlueprintLibrary.SetInputMode_GameOnly` self)
  (set `self.bShowMouseCursor` false))

(event `self.ShowGameOverHUD`
  (params (WinnerIndex :type Integer))
  ;[1 1 1] WinScreen
  (bind _asstolemates_game_instance (cast `StolematesGameInstance` (`GameplayStatics.GetGameInstance`)))
  (switch `EMatchType` (`StolematesGameInstance.MatchType` _asstolemates_game_instance)
    (:`Local`
      (if (== (`GameplayStatics.GetPlayerController` WinnerIndex) self)
        (bind _returnvalue (`|CreateWidget` "/Game/Blueprints/Win.Win_C" self))
        (set `/Game/Blueprints/Win.WinnerIndex` WinnerIndex _returnvalue)
        (`UserWidget.AddToViewport` _returnvalue 0)
        (`/Game/Blueprints/Win.InitializeFocus` _returnvalue)))
    (:`Online`
      (bind _returnvalue_2 (`|CreateWidget` "/Game/Blueprints/Win.Win_C" self))
      (set `/Game/Blueprints/Win.WinnerIndex` WinnerIndex _returnvalue_2)
      (`UserWidget.AddToViewport` _returnvalue_2 0)
      (`/Game/Blueprints/Win.InitializeFocus` _returnvalue_2))))

(event `self.ReturnToMainMenuRequested`
  ;[1 1 1] mainMenu
  (bind _asstolemates_game_instance (cast `StolematesGameInstance` (`GameplayStatics.GetGameInstance`)))
  (`StolematesGameInstance.ReturnToMainMenu` _asstolemates_game_instance))

(event `self.SetMatchStartMessage`
  (params (Message :type String) (bVisible :type Boolean))
  (bind _matchstartmessagewidget (`self.MatchStartMessageWidget`))
  ;[1 1 1] WaitingForPlayers
  (if bVisible
    (`/Engine/EditorBlueprintResources/StandardMacros.IsValid` _matchstartmessagewidget
      (:`Is Valid`
        (`Widget.RemoveFromParent` _matchstartmessagewidget))
      (:`Is Not Valid`
        _))
    (bind _returnvalue (`|CreateWidget` "/Game/Blueprints/WaitingForPlayers.WaitingForPlayers_C" self))
    (bind _output_get (set `self.MatchStartMessageWidget` _returnvalue))
    (`UserWidget.AddToViewport` _output_get 999)
    (`self.MarkMatchStartReady`)
    (else
      (`/Engine/EditorBlueprintResources/StandardMacros.IsValid` _matchstartmessagewidget
        (:`Is Valid`
          (`Widget.RemoveFromParent` _matchstartmessagewidget)
          (set `self.MatchStartMessageWidget` null))))))

(event `self.ShowOnlinePauseMenu`
  (params (bCanResume :type Boolean))
  (bind _currentpausemenu (`self.CurrentPauseMenu`))
  ;[1 1 1] ShowPause
  (`/Engine/EditorBlueprintResources/StandardMacros.IsValid` _currentpausemenu
    (:`Is Valid`
      (`Widget.RemoveFromParent` _currentpausemenu))
    (:`Is Not Valid`
      _))
  (bind _returnvalue (`|CreateWidget` "/Game/Blueprints/PauseMenu.PauseMenu_C"))
  (set `/Game/Blueprints/PauseMenu.CanResume` bCanResume _returnvalue)
  (set `self.CurrentPauseMenu` _returnvalue)
  (`UserWidget.AddToViewport` _returnvalue 0)
  (`WidgetBlueprintLibrary.SetInputMode_GameAndUIEx` null _returnvalue "DoNotLock" false)
  (set `self.bShowMouseCursor` true))

(event `self.UpdatePowerUpHUD`
  (params (PlayerIndex :type Integer) (PowerUpIndex :type Integer))
  (bind _hudref (`self.HUDRef`))
  ;[1 1 1] PowerupHUD
  (`/Engine/EditorBlueprintResources/StandardMacros.IsValid` _hudref
    (:`Is Valid`
      (`/Game/Blueprints/HUD.Update Player PowerUp` _hudref PowerUpIndex PlayerIndex))))

(event `self.HideOnlinePauseMenu`
  (bind _currentpausemenu (`self.CurrentPauseMenu`))
  ;[1 1 1] HidePause
  (`/Engine/EditorBlueprintResources/StandardMacros.IsValid` _currentpausemenu
    (:`Is Valid`
      (`Widget.RemoveFromParent` _currentpausemenu)
      (set `self.CurrentPauseMenu` null)
      (`WidgetBlueprintLibrary.SetInputMode_GameOnly` null)
      (set `self.bShowMouseCursor` false))))

(fn `UserConstructionScript`)