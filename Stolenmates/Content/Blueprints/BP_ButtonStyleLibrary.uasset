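; Button style helper library with one function, GetButtonTextColor, which derives a text color from a button's current state.
; It checks enabled, pressed and hovered in that order and returns the matching Disabled, Pressed, Hovered or Normal brush tint from the button's WidgetStyle.
; The color comes from the button's own style brushes, so no separate text palette is involved.
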(fn `GetButtonTextColor`
  (params (`Button Reference` :type "Button Object Reference"))
  (returns (`Slate Color` :type "SlateColor Structure"))
  (bind _widgetstyle (`Button.WidgetStyle` `Button Reference`))
  (if (`Widget.bIsEnabled` `Button Reference`)
    (if (`Button.IsPressed` `Button Reference`)
      (return (`.TintColor` (break `SlateBrush` (`.Pressed` (break `ButtonStyle` _widgetstyle)))))
      (elif (`Widget.IsHovered` `Button Reference`)
        (return (`.TintColor` (break `SlateBrush` (`.Hovered` (break `ButtonStyle` _widgetstyle)))))
        (else
          (return (`.TintColor` (break `SlateBrush` (break `ButtonStyle` _widgetstyle)))))))
    (else
      (return (`.TintColor` (break `SlateBrush` (`.Disabled` (break `ButtonStyle` _widgetstyle))))))))