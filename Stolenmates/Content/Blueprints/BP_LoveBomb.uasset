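; BP_LoveBomb is a player ability that launches a BP_Tracking actor at the nearest other player.
; On FireAbility it takes the player list from StolenmatesGameModeBase, seeds a candidate with one loop, then finds the closest by distance in a second.
; It spawns the tracker at the user's transform with that player as Target and the user as Creator, then sets the user's ability to BOXABILITY.
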(event `self.fireAbility`
  (params (abilityUser :type "StolenmatesPlayer Object Reference"))
  (bind _asbp_player (cast `/Game/Blueprints/BP_Player` abilityUser))
  (bind _asstolenmates_game_mode_base (cast `StolenmatesGameModeBase` (`GameplayStatics.GetGameMode`)))
  (bind _returnvalue (`StolenmatesGameModeBase.getPlayers` _asstolenmates_game_mode_base))
  (for _array_element _returnvalue
    (bind _asbp_player_2 (cast `/Game/Blueprints/BP_Player` _array_element))
    (if (!= _asbp_player_2 _asbp_player)
      (bind _output_get (set `self.ClosestPlayer` _asbp_player_2))
      (set `self.ClosestTransform` (`self.K2_GetActorLocation` _output_get))))
  (for _array_element_2 _returnvalue
    (bind _asbp_player_3 (cast `/Game/Blueprints/BP_Player` _array_element_2))
    (if (!= _asbp_player_3 _asbp_player)
      (bind _returnvalue_2 (`self.K2_GetActorLocation` _asbp_player))
      (if (< (`KismetMathLibrary.Vector_Distance` (`self.K2_GetActorLocation` _asbp_player_3) _returnvalue_2) (`KismetMathLibrary.Vector_Distance` _returnvalue_2 (`self.ClosestTransform`)))
        (bind _output_get_2 (set `self.ClosestPlayer` _asbp_player_3))
        (set `self.ClosestTransform` (`self.K2_GetActorLocation` _output_get_2)))))
  (`|SpawnActorFromClass` "/Game/Blueprints/BP_Tracking.BP_Tracking_C" (`self.GetTransform` _asbp_player) "AdjustIfPossibleButAlwaysSpawn" "OverrideRootScale" null _asbp_player (`self.ClosestPlayer`) null)
  (`StolenmatesPlayer.SetAbility` _asbp_player "ITEM_BOX_ABILITY" null))

(fn `UserConstructionScript`)