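; BP_FollowSpline is a temporary actor that carries the player along a spline path over a set travel time.
; On BeginPlay it stuns the BP_Player follower for that duration and starts a looping timer at roughly 60 Hz, instead of using Tick.
; Each step teleports the follower to the elapsed fraction of spline length, using location only, then the actor destroys itself when time runs out.
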(event `self.ReceiveBeginPlay`
  (bind _asbp_player (cast `/Game/Blueprints/BP_Player` (`self.Follower`)))
  (`StolenmatesPlayer.StunPlayer` _asbp_player (`self.Total Travel Time`))
  (bind _returnvalue (`KismetSystemLibrary.K2_SetTimerDelegate` (delegate `Follow Spline`) 0.016 true)))

(event `Follow Spline`
  (set `self.Elapsed Time` (+ 0.016 (`self.Elapsed Time`)))
  (`self.K2_SetActorTransform` (`self.Follower`) (`KismetMathLibrary.Conv_VectorToTransform` (`SplineComponent.GetLocationAtDistanceAlongSpline` (`self.Path to follow`) (* (`SplineComponent.GetSplineLength` (`self.Path to follow`)) (/ (`self.Elapsed Time`) (`self.Total Travel Time`))) "World")) false true)
  (if (>= (`self.Elapsed Time`) (`self.Total Travel Time`))
    (`KismetSystemLibrary.K2_ClearAndInvalidateTimerHandle` (stale `self.ReceiveBeginPlay` _returnvalue))
    (`self.K2_DestroyActor`)))

(fn `UserConstructionScript`)